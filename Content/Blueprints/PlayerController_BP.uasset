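; Player-controlled third-person pawn, despite the PlayerController name, handling camera orbit and movement through Enhanced Input.
; BeginPlay adds the player input mapping context for player 0.
; Camera input yaws the spring arm and Cylinder together in world space and pitches only the arm locally, scaled by rotation speed.
; Movement input follows the camera's unflattened forward and right vectors, scaled by movement speed.
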(event `self.ReceiveBeginPlay`
  (`self.InitMappingContext`))

(event `EnhancedInput|/Game/Inputs/Actions/CameraMovement_IA`
  (params (ActionValue :type "Vector2D Structure") (ElapsedSeconds :type "Float (double-precision)") (TriggeredSeconds :type "Float (double-precision)") (InputAction :type "InputAction Object Reference" :default "/Game/Inputs/Actions/CameraMovement_IA.CameraMovement_IA"))
  (:`Triggered`
    (`self.RotateThirdPersonCamera` ActionValue_X ActionValue_Y)))

(event `EnhancedInput|/Game/Inputs/Actions/PlayerMovement_IA`
  (params (ActionValue :type "Vector2D Structure") (ElapsedSeconds :type "Float (double-precision)") (TriggeredSeconds :type "Float (double-precision)") (InputAction :type "InputAction Object Reference" :default "/Game/Inputs/Actions/PlayerMovement_IA.PlayerMovement_IA"))
  (bind _camera (`self.Camera`))
  (bind _movementspeed (`self.MovementSpeed`))
  (:`Triggered`
    (`self.AddMovementInput` (`SceneComponent.GetForwardVector` _camera) (* ActionValue_Y _movementspeed))
    (`self.AddMovementInput` (`SceneComponent.GetRightVector` _camera) (* _movementspeed ActionValue_X))))

(fn `InitMappingContext`
  (`EnhancedInputSubsystemInterface.AddMappingContext` (pcsubsystem `EnhancedInputLocalPlayerSubsystem` (`GameplayStatics.GetPlayerController` 0)) "/Game/Inputs/PlayerInput_IMC.PlayerInput_IMC" 0 (struct)))

(fn `RotateThirdPersonCamera`
  (params (A :type "Float (double-precision)") (B :type "Float (double-precision)"))
  (bind _springarm (`self.SpringArm`))
  (bind _camrotationspeed (`self.CamRotationSpeed`))
  (`SceneComponent.K2_AddWorldRotation` _springarm (`KismetMathLibrary.MakeRotator` 0.0 0.0 (* A _camrotationspeed)) false false)
  (`SceneComponent.K2_AddWorldRotation` (`self.Cylinder`) (`KismetMathLibrary.MakeRotator` 0.0 0.0 (* A _camrotationspeed)) false false)
  (`SceneComponent.K2_AddLocalRotation` _springarm (`KismetMathLibrary.MakeRotator` 0.0 (* B _camrotationspeed)) false false))

(fn `UserConstructionScript`)