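; Light beam actor for a light puzzle that visually extends to whatever it hits and links to that puzzle element.
; UpdateLightBeam line-traces on Visibility, ignoring the holder (parent actor by default), and Z-scales Origin to the hit or the CutOff length.
; Changed hits send disconnect and connect messages to the actors, storing only accepted connections.
; SetRayEnabled toggles beam visibility and connects or disconnects the stored element.
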(event `self.ReceiveBeginPlay`
  (set `self.RayHolder` (`self.GetParentActor`)))

(fn `SetRayEnabled`
  (params (enabled :type Boolean))
  (bind _hitelement (`self.HitElement`))
  (`SceneComponent.SetVisibility` (`self.Ray`) enabled false)
  (`/Engine/EditorBlueprintResources/StandardMacros.IsValid` _hitelement
    (:`Is Valid`
      (if enabled
        (message `/Game/LightPuzzles/LightPuzzleElement_IF.Connect` _hitelement self)
        (else
          (message `/Game/LightPuzzles/LightPuzzleElement_IF.Disconnect` _hitelement))))))

(fn `SetRayHolder`
  (params (holder :type "Actor Object Reference"))
  (set `self.RayHolder` holder))

(fn `UpdateHitPuzzleElement`
  (params (hit_actor :type "Actor Object Reference"))
  (bind _hitelement (`self.HitElement`))
  (if (!= hit_actor (`self.HitElement`))
    ;[1 1 1] Disconnect Current
    (`/Engine/EditorBlueprintResources/StandardMacros.IsValid` _hitelement
      (:`Is Valid`
        (message `/Game/LightPuzzles/LightPuzzleElement_IF.Disconnect` _hitelement))
      (:`Is Not Valid`
        _))
    ;[1 1 1] Connect New
    (`/Engine/EditorBlueprintResources/StandardMacros.IsValid` hit_actor
      (:`Is Valid`
        (bind _successful (message `/Game/LightPuzzles/LightPuzzleElement_IF.Connect` hit_actor self))
        (if _successful
          (set `self.HitElement` hit_actor :!label _label) ; Store new value
          (else
            (set `self.HitElement` (`self.NULL_HitElement`)) ; if the connection was not successful, do not store the other element
          )))
      (:`Is Not Valid`
        (goto _label)))))

(fn `UpdateLightBeam`
  (bind _origin (`self.Origin`))
  (bind _returnvalue (`SceneComponent.K2_GetComponentLocation` _origin))
  (bind _outhit (`KismetSystemLibrary.LineTraceSingle` _returnvalue (+ _returnvalue (* (`SceneComponent.GetUpVector` _origin) (* (`self.CutOff`) 100.0))) "TraceTypeQuery1" false (`|MakeArray` (`self.RayHolder`))))
  (bind (_bblockinghit _binitialoverlap _time _distance _location _impactpoint _normal _impactnormal _physmat _hitactor) (`GameplayStatics.BreakHitResult` _outhit))
  (if _bblockinghit
    ;[1 1 1] If something is hit, the ray should stop at that object. Update the hit element
    (`SceneComponent.SetWorldScale3D` (`self.Origin`) (`KismetMathLibrary.MakeVector` 1.0 1.0 (/ (`KismetMathLibrary.VSize` (- (`SceneComponent.K2_GetComponentLocation` (`self.Origin`)) _location)) 100.0)))
    (`self.UpdateHitPuzzleElement` _hitactor)
    (else
      ;[1 1 1] If nothing is hit, ray has maximum length. Update the hit element
      (`SceneComponent.SetWorldScale3D` (`self.Origin`) (`KismetMathLibrary.MakeVector` 1.0 1.0 (`self.CutOff`)))
      (`self.UpdateHitPuzzleElement` (`self.NULL_HitElement`)))))

(fn `UserConstructionScript`)