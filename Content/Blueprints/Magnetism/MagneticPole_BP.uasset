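; Magnetic pole actor that pulls on or pushes away physics components within its spherical action range.
; Every Tick, ApplyInfluence applies equal and opposite half-forces at the centers of mass of the pole and each overlapping component.
; Force falls off quadratically to zero at the sphere radius.
; Polarity comes from material slot 0, set on construction: matching materials repel, differing ones attract.
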(event `self.ReceiveTick`
  (params (DeltaSeconds :type "Float (single-precision)"))
  (bind _actionrange (`self.ActionRange`))
  (`self.ApplyInfluence` (`self.Pole`) _actionrange (`SphereComponent.SphereRadius` _actionrange)))

(fn `ApplyInfluence`
  (params (Pole :type "PrimitiveComponent Object Reference") (ActionRange :type "PrimitiveComponent Object Reference") (MaxDistance :type "Float (double-precision)"))
  (locals (mPole :type "PrimitiveComponent Object Reference") (mActionRange :type "PrimitiveComponent Object Reference") (mForeignPole :type "PrimitiveComponent Object Reference") (mMaxDistance :type "Float (double-precision)"))
  (bind _mmaxdistance (`local.mMaxDistance`))
  (bind _returnvalue (`PrimitiveComponent.GetCenterOfMass` (`local.mForeignPole`) "None"))
  (bind _returnvalue_2 (`PrimitiveComponent.GetCenterOfMass` (`local.mPole`) "None"))
  (bind _returnvalue_3 (- _returnvalue_2 _returnvalue))
  (bind _returnvalue_4 (/ (* (* (`KismetMathLibrary.Normal` _returnvalue_3) (* (`self.mMagneticForce`) (`KismetMathLibrary.Square` (/ (- _mmaxdistance (`KismetMathLibrary.FClamp` (`KismetMathLibrary.VSize` _returnvalue_3) 0.0 _mmaxdistance)) _mmaxdistance)))) (select `bool` (!= (`PrimitiveComponent.GetMaterial` (`local.mPole`) 0) (`PrimitiveComponent.GetMaterial` (`local.mForeignPole`) 0)) :`false` -1.0 :`true` 1.0 :!type "Float (single-precision)")) 2.0))
  (set `local.mPole` Pole)
  (set `local.mActionRange` ActionRange)
  (set `local.mMaxDistance` MaxDistance)
  (for _array_element (`PrimitiveComponent.GetOverlappingComponents` (`local.mActionRange`))
    (bind _output_get (set `local.mForeignPole` _array_element))
    (if (!= _output_get (`local.mPole`))
      (`PrimitiveComponent.AddForceAtLocation` (`local.mForeignPole`) _returnvalue_4 _returnvalue "None")
      (`PrimitiveComponent.AddForceAtLocation` (`local.mPole`) (* _returnvalue_4 -1.0) _returnvalue_2 "None"))))

(fn `UserConstructionScript`
  (`PrimitiveComponent.SetMaterial` (`self.Pole`) 0 (`self.Material`)))