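; Light puzzle converger that emits its own beam only once every required incoming side (left, back, right) is lit.
; DetermineRayDirection identifies the side by comparing the incoming ray's forward vector with the Cube's axes, within a small tolerance.
; Connect records hits, accepts rays only on enabled sides, and switches on the child LightBeam_BP when all those are hit.
; Disconnect clears that side's hit and always switches the output beam off.
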(event `self.ReceiveBeginPlay`
  (bind _aslight_beam_bp (cast `/Game/LightPuzzles/LightBeam_BP` (`ChildActorComponent.ChildActor` (`self.LightBeam_BP`))))
  (`/Game/LightPuzzles/LightBeam_BP.SetRayEnabled` _aslight_beam_bp false)
  (set `self.HitLeft` false)
  (set `self.HitBack` false)
  (set `self.HitRight` false))

(event `/Game/LightPuzzles/LightPuzzleElement_IF.Disconnect`
  (params (OtherRay :type "Actor Object Reference"))
  (bind _aslight_beam_bp (cast `/Game/LightPuzzles/LightBeam_BP` (`ChildActorComponent.ChildActor` (`self.LightBeam_BP`))))
  (`/Game/LightPuzzles/LightBeam_BP.SetRayEnabled` _aslight_beam_bp false)
  (bind _direction (`self.DetermineRayDirection` OtherRay))
  (if (== (break `IntVector` _direction) 1)
    (set `self.HitLeft` false)
    (elif (== (`.Y` (break `IntVector` _direction)) 1)
      (set `self.HitBack` false)
      (elif (== (`.Z` (break `IntVector` _direction)) 1)
        (set `self.HitRight` false)))))

(fn `Connect`
  (params (OtherRay :type "Actor Object Reference"))
  (returns (successful :type Boolean))
  (bind _incoming_hit (`self.SetHitDirection` OtherRay))
  (if _incoming_hit
    (if (and (or (`self.HitLeft`) (not (`self.IncomingLeft`))) (or (`self.HitBack`) (not (`self.IncomingBack`))) (or (`self.HitRight`) (not (`self.IncomingRight`))))
      (bind _aslight_beam_bp (cast `/Game/LightPuzzles/LightBeam_BP` (`ChildActorComponent.ChildActor` (`self.LightBeam_BP`))))
      (`/Game/LightPuzzles/LightBeam_BP.SetRayEnabled` _aslight_beam_bp true)
      (`/Game/LightPuzzles/LightBeam_BP.UpdateLightBeam` _aslight_beam_bp))
    (return true)
    (else
      (return false))))

(fn `DetermineRayDirection`
  (params (incoming_ray :type "Actor Object Reference"))
  (returns (direction :type "IntVector Structure"))
  (bind _returnvalue (`KismetMathLibrary.NegateVector` (`self.GetActorForwardVector` incoming_ray)))
  (if (== _returnvalue (`KismetMathLibrary.NegateVector` (`SceneComponent.GetForwardVector` (`self.Cube`))) :`ErrorTolerance` 0.1)
    (return (make `IntVector` 0 1))
    (elif (== _returnvalue (`SceneComponent.GetRightVector` (`self.Cube`)) :`ErrorTolerance` 0.1)
      (return (make `IntVector` 0 0 1))
      (elif (== _returnvalue (`KismetMathLibrary.NegateVector` (`SceneComponent.GetRightVector` (`self.Cube`))) :`ErrorTolerance` 0.1)
        (return (make `IntVector` 1))))))

(fn `SetHitDirection`
  (params (`incoming ray` :type "Actor Object Reference"))
  (returns (`incoming hit` :type Boolean))
  (bind _direction (`self.DetermineRayDirection` `incoming ray`))
  (if (== (break `IntVector` _direction) 1)
    (set `self.HitLeft` true)
    (return (`self.IncomingLeft`))
    (elif (== (`.Y` (break `IntVector` _direction)) 1)
      (set `self.HitBack` true)
      (return (`self.IncomingBack`))
      (elif (== (`.Z` (break `IntVector` _direction)) 1)
        (set `self.HitRight` true)
        (return (`self.IncomingRight`))
        (else
          (return false))))))

(fn `UserConstructionScript`)