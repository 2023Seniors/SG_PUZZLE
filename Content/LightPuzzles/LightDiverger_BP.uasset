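; LightDiverger_BP is a light puzzle piece that splits an incoming beam into left, front and right output beams.
; Connect accepts the other actor only if its forward vector nearly matches the Cube's, then enables and updates each child LightBeam_BP selected by the Left, Front and Right flags.
; It returns whether the connection succeeded.
; BeginPlay and Disconnect share the logic that switches all three output rays off.
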(event `self.ReceiveBeginPlay`
  (bind _aslight_beam_bp (cast `/Game/LightPuzzles/LightBeam_BP` (`ChildActorComponent.ChildActor` (`self.LightBeam_Left`)) :!label _label))
  (`/Game/LightPuzzles/LightBeam_BP.SetRayEnabled` _aslight_beam_bp false)
  (bind _aslight_beam_bp_2 (cast `/Game/LightPuzzles/LightBeam_BP` (`ChildActorComponent.ChildActor` (`self.LightBeam_Front`))))
  (`/Game/LightPuzzles/LightBeam_BP.SetRayEnabled` _aslight_beam_bp_2 false)
  (bind _aslight_beam_bp_3 (cast `/Game/LightPuzzles/LightBeam_BP` (`ChildActorComponent.ChildActor` (`self.LightBeam_Right`))))
  (`/Game/LightPuzzles/LightBeam_BP.SetRayEnabled` _aslight_beam_bp_3 false))

(event `self.ReceiveTick`
  (params (DeltaSeconds :type "Float (single-precision)")))

(event `/Game/LightPuzzles/LightPuzzleElement_IF.Disconnect`
  (goto _label))

(fn `ComputeIndividualLightBeam`
  (params (beam :type "ChildActorComponent Object Reference"))
  (bind _aslight_beam_bp (cast `/Game/LightPuzzles/LightBeam_BP` (`ChildActorComponent.ChildActor` beam)))
  (`/Game/LightPuzzles/LightBeam_BP.SetRayEnabled` _aslight_beam_bp true)
  (`/Game/LightPuzzles/LightBeam_BP.UpdateLightBeam` _aslight_beam_bp))

(fn `Connect`
  (params (Other :type "Actor Object Reference"))
  (returns (successful :type Boolean))
  (if (== (`self.GetActorForwardVector` Other) (`SceneComponent.GetForwardVector` (`self.Cube`)) :`ErrorTolerance` 0.1)
    (if (`self.Right`)
      (`self.ComputeIndividualLightBeam` (`self.LightBeam_Right`)))
    (if (`self.Front`)
      (`self.ComputeIndividualLightBeam` (`self.LightBeam_Front`)))
    (if (`self.Left`)
      (`self.ComputeIndividualLightBeam` (`self.LightBeam_Left`)))
    (return true)
    (else
      (return false))))

(fn `UserConstructionScript`)