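; InteractableBlockBP is an interactable block actor whose Cube spins left or right when RotateLeft or RotateRight is called.
; Each event is gated by IsSelected, which acts as a busy lock so new rotation calls are ignored mid-animation.
; Per-direction timelines play from start, setting the Cube's relative yaw directly from their curve value, then clear the lock and print a debug message.
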(event `self.ReceiveTick`
  (params (DeltaSeconds :type "Float (single-precision)")))

(event `/Game/Interfaces/BlockInteractInterface.RotateRight`
  (if (not (`self.IsSelected`))
    (set `self.IsSelected` true)
    (bind (_direction _rotationright) (`Timeline|RightRotationTimeline` :!via `PlayFromStart`)
      (:`Update`
        (`SceneComponent.K2_SetRelativeRotation` (`self.Cube`) (`KismetMathLibrary.MakeRotator` 0.0 0.0 _rotationright) false false))
      (:`Finished`
        (set `self.IsSelected` false)
        (`KismetSystemLibrary.PrintString` "Ended Rotation")))))

(event `/Game/Interfaces/BlockInteractInterface.RotateLeft`
  (if (not (`self.IsSelected`))
    (set `self.IsSelected` true)
    (bind (_direction _leftrotation) (`Timeline|LeftRotationTimeline` :!via `PlayFromStart`)
      (:`Update`
        (`SceneComponent.K2_SetRelativeRotation` (`self.Cube`) (`KismetMathLibrary.MakeRotator` 0.0 0.0 _leftrotation) false false))
      (:`Finished`
        (set `self.IsSelected` false)
        (`KismetSystemLibrary.PrintString` "Ended Rotation")))))

(fn `UserConstructionScript`)